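; Menu layer actor that shows a screen-space billboard material and shifts it with the mouse cursor, apparently for a parallax effect.
; BeginPlay adds the billboard element with slightly padded base dimensions.
; Every Tick normalizes the cursor position around the viewport center, scales it by MousePositionModifier, and sets the actor's Y (inverted) and Z (plus ZOffset), leaving X unchanged.
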(event `self.ReceiveBeginPlay`
  (`MaterialBillboardComponent.AddElement` (`self.MaterialBillboard`) (`self.BillboardMaterial`) null true (+ (`self.BaseSizeX`) 0.1) (+ (`self.BaseSizeY`) 0.1) null))

(event `self.ReceiveTick`
  (params (DeltaSeconds :type "Float (single-precision)"))
  (bind _mousepositionmodifier (`self.MousePositionModifier`))
  (bind (_locationx _locationy) (`PlayerController.GetMousePosition` (`GameplayStatics.GetPlayerController` 0)))
  (bind (_x _y) (`KismetMathLibrary.BreakVector2D` (/ (`KismetMathLibrary.MakeVector2D` _locationx _locationy) (/ (`WidgetLayoutLibrary.GetViewportSize`) 2.0))))
  (`self.K2_SetActorLocation` (`KismetMathLibrary.MakeVector` (.x (`self.K2_GetActorLocation`)) (* (- (* _mousepositionmodifier _x) _mousepositionmodifier) -1.0) (+ (- (* _mousepositionmodifier _y) _mousepositionmodifier) (`self.ZOffset`)))))

(fn `UserConstructionScript`)