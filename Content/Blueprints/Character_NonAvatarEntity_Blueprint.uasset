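; Character blueprint for non-avatar entities, handling hurricane collisions with avatar characters.
; When its box component overlaps a box on a Pathfinder character, it skips components named as attack traces and requires an avatar AI controller.
; Qualifying overlaps call HurricaneOnAvatarCollision with that character.
; A delayed step enabling query-only box collision for the Hurricane entity type is left disconnected and never runs.
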(event `self.ReceiveBeginPlay`)

(event `self.BoxComponent.OnComponentBeginOverlap`
  (params (OverlappedComponent :type "PrimitiveComponent Object Reference") (OtherActor :type "Actor Object Reference") (OtherComp :type "PrimitiveComponent Object Reference") (OtherBodyIndex :type Integer) (bFromSweep :type Boolean) (SweepResult :type "HitResult Structure (by ref)"))
  (bind _ascharacter_pathfinder (cast `Character_Pathfinder` OtherActor))
  (bind _asbox_collision (cast `BoxComponent` OtherComp))
  (if (not (`KismetStringLibrary.Contains` (`KismetSystemLibrary.GetObjectName` _asbox_collision) "AttackTrace"))
    (cast `AIController_Avatar` (`AIBlueprintHelperLibrary.GetAIController` _ascharacter_pathfinder))
    (`self.HurricaneOnAvatarCollision` _ascharacter_pathfinder)))

(fn `UserConstructionScript`)