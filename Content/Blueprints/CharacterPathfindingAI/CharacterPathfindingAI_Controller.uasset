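; AI controller that moves characters by pathfinding, running a behavior tree and enabling movement replication on possess.
; AIMoveToLocation_Server writes the destination into the TargetLocation blackboard key.
; A move-completed handler updates the state of every grid tile actor, but its binding and Invalid-result guard are disconnected.
; Debug path-sphere drawing is also disconnected, leaving Tick empty.
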(event `self.ReceivePossess`
  (params (PossessedPawn :type "Pawn Object Reference"))
  ;[1 1 1] Run the AI Pathfinding BehaviourTree
  (`self.RunBehaviorTree` "/Game/Blueprints/CharacterPathfindingAI/CharacterPathfindingAI_BehaviourTree.CharacterPathfindingAI_BehaviourTree")
  (`self.SetReplicateMovement` true))

(event `self.ReceiveTick`
  (params (DeltaSeconds :type "Float (single-precision)"))
  ;[1 1 1] Debug Draw Path
)

(event `ReceiveMoveCompleted_Event` :!signature `self.ReceiveMoveCompleted`
  (params (RequestID :type "AIRequestID Structure") (Result :type "EPathFollowingResult Enum" :default "Success"))
  ;[1 1 1] Update GridTiles upon Avatars finishing movement
  (bind _outactors (`GameplayStatics.GetAllActorsOfClass` "/Game/Blueprints/Actor_GridTile_Blueprint.Actor_GridTile_Blueprint_C"))
  (for _array_element _outactors
    (`Actor_GridTile.UpdateGridTileState` _array_element)))

(event `AIMoveToLocation_Server`
  (params (Location :type "Vector Structure"))
  (`BlackboardComponent.SetValueAsVector` (`self.Blackboard`) "TargetLocation" Location))

(fn `UserConstructionScript`)