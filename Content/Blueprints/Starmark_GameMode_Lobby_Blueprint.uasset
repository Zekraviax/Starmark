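; Game mode for the Starmark multiplayer lobby, handling player joins, lobby roster updates and launch into the arena.
; On PostLogin it spawns and possesses a static pawn, tracks the controller, notifies it, and updates the first player's ready status with the server flag.
; UpdatePlayerLobbyWidgets collects names and ready states from the game state's player array and sends them to each tracked lobby controller.
; LaunchGame server-travels to the MultiplayerArena level.
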(event `self.K2_PostLogin`
  (params (NewPlayer :type "PlayerController Object Reference"))
  (bind _returnvalue (`KismetSystemLibrary.IsServer`))
  (bind _returnvalue_2 (`|SpawnActorFromClass` "/Game/Blueprints/PlayerPawn_Static_Blueprint.PlayerPawn_Static_Blueprint_C" (`KismetMathLibrary.MakeTransform` (0.0 0.0 0.0)) "Undefined" "OverrideRootScale" null null))
  (`Controller.Possess` NewPlayer _returnvalue_2)
  (`KismetArrayLibrary.Array_Add` (`self.PlayerControllersArray`) NewPlayer)
  (bind _asplayer_controller_lobby_blueprint (cast `/Game/Blueprints/PlayerController_Lobby_Blueprint` NewPlayer))
  (`PlayerController_Lobby.PlayerJoinedMultiplayerLobby` _asplayer_controller_lobby_blueprint)
  (if _returnvalue
    (`/Game/Blueprints/Starmark_PlayerState_Blueprint.BlueprintUpdateReadyStatus` (cast `/Game/Blueprints/Starmark_PlayerState_Blueprint` (`Controller.PlayerState` (`GameplayStatics.GetPlayerController` 0)) :!pure true) _returnvalue)))

(event `LaunchGame`
  (`KismetSystemLibrary.ExecuteConsoleCommand` "servertravel /Game/Levels/MultiplayerArena" (`GameplayStatics.GetPlayerController` 0)))

(event `UpdatePlayerLobbyWidgets`
  ;[1 1 1] Lobby Update
  (`KismetArrayLibrary.Array_Clear` (`self.Temporary_PlayerNamesArray`))
  (`KismetArrayLibrary.Array_Clear` (`self.Temporary_PlayerReadyStatusesArray`))
  (for _array_element (`GameStateBase.PlayerArray` (cast `/Game/Blueprints/Starmark_GameState_Blueprint` (`GameplayStatics.GetGameState`) :!pure true))
    (bind _asstarmark_player_state_blueprint (cast `/Game/Blueprints/Starmark_PlayerState_Blueprint` _array_element :!pure true))
    (`KismetArrayLibrary.Array_Add` (`self.Temporary_PlayerNamesArray`) (`Starmark_PlayerState.ReplicatedPlayerName` _asstarmark_player_state_blueprint))
    (`KismetArrayLibrary.Array_Add` (`self.Temporary_PlayerReadyStatusesArray`) (`/Game/Blueprints/Starmark_PlayerState_Blueprint.BlueprintPlayerReadyStatus` _asstarmark_player_state_blueprint)))
  (for _array_element_2 (`self.PlayerControllersArray`)
    (`PlayerController_Lobby.Client_UpdatePlayersInLobby` (cast `/Game/Blueprints/PlayerController_Lobby_Blueprint` _array_element_2 :!pure true) (`self.Temporary_PlayerNamesArray`) (`self.Temporary_PlayerReadyStatusesArray`) true)))

(fn `UserConstructionScript`)