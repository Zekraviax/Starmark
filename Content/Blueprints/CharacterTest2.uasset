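; CharacterTest2 is a selectable test character that shows a cursor-hover highlight and takes move targets through GraphAStar interface events.
; A dynamic material on its selection decal turns white on hover and green on SelectPawn, and hover changes are skipped while selected.
; SetTargetLocation writes the destination to the AI controller's blackboard for the behaviour tree to handle movement.
; CursorLocation is an empty stub.
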(event `self.ReceiveBeginPlay`
  ;[1 1 1] Create OnCursorHoverOver Material
  (bind _returnvalue (`DecalComponent.CreateDynamicMaterialInstance` (`self.SelectionDecal`)))
  (set `self.DynamicMaterialReference` _returnvalue))

(event `self.ReceiveActorBeginCursorOver`
  ;[1 1 1] OnCursorOver Events
  (if (not (`self.IsSelected`))
    (`SceneComponent.SetVisibility` (`self.SelectionDecal`) true false)
    (`MaterialInstanceDynamic.SetVectorParameterValue` (`self.DynamicMaterialReference`) "Colour" (struct :`R` 1.0 :`G` 1.0 :`B` 1.0 :`A` 1.0))))

(event `self.ReceiveActorEndCursorOver`
  ;[1 1 1] OnCursorOver Events
  (if (not (`self.IsSelected`))
    (`SceneComponent.SetVisibility` (`self.SelectionDecal`) false false)))

(event `/Game/Blueprints/Interfaces/BlueprintInterface_GraphAStar.CursorLocation`
  (params (Location :type "Vector Structure"))
  ;[1 1 1] GraphAStar Blueprint Interface Implementations
)

(event `/Game/Blueprints/Interfaces/BlueprintInterface_GraphAStar.SelectPawn`
  (params (IsSelected :type Boolean))
  ;[1 1 1] GraphAStar Blueprint Interface Implementations
  (set `self.IsSelected` IsSelected)
  (`MaterialInstanceDynamic.SetVectorParameterValue` (`self.DynamicMaterialReference`) "Colour" (struct :`G` 1.0 :`A` 1.0)))

(event `/Game/Blueprints/Interfaces/BlueprintInterface_GraphAStar.SetTargetLocation`
  (params (TargetLocation :type "Vector Structure"))
  (bind _returnvalue (`AIBlueprintHelperLibrary.GetBlackboard` (`AIBlueprintHelperLibrary.GetAIController` self)))
  ;[1 1 1] Use the Characters AI Behaviour Tree to move it
  (`/Engine/EditorBlueprintResources/StandardMacros.IsValid` _returnvalue
    (:`Is Valid`
      (`BlackboardComponent.SetValueAsVector` _returnvalue "TargetLocation" TargetLocation))
    (:`Is Not Valid`
      (`KismetSystemLibrary.PrintString` "BB Not Valid"))))

(fn `UserConstructionScript`)