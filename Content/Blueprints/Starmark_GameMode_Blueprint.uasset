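; Starmark game mode Blueprint that handles multiplayer player login and end-of-battle session teardown.
; PostLogin casts each new player to PlayerController_Base_Blueprint and passes it to OnPlayerPostLogin.
; EndOfBattle waits briefly, destroys the session through the first player controller, and on success calls EndOfSession on the stored player controllers.
; DisplayErrorMessage shows error text with a debug PrintString.
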(event `self.K2_PostLogin`
  (params (NewPlayer :type "PlayerController Object Reference"))
  ;[1 1 1] Mtultiplayer Functions
  (bind _asplayer_controller_base_blueprint (cast `/Game/Blueprints/PlayerController_Base_Blueprint` NewPlayer))
  (`self.OnPlayerPostLogin` _asplayer_controller_base_blueprint))

(event `self.EndOfBattle`
  ;[1 1 1] Mtultiplayer Functions
  (`KismetSystemLibrary.Delay` 3.0)
  (`DestroySessionCallbackProxy.DestroySession` (`GameplayStatics.GetPlayerController` 0)
    (:`OnSuccess`
      (for _array_element (`self.PlayerControllerReferences`)
        (bind _asplayer_controller_base_blueprint (cast `/Game/Blueprints/PlayerController_Base_Blueprint` _array_element))
        (`/Game/Blueprints/PlayerController_Base_Blueprint.EndOfSession` _asplayer_controller_base_blueprint)))))

(fn `UserConstructionScript`)