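; Player state Blueprint for Starmark that handles lobby ready status and lobby widget refreshes.
; The ready-status event marks the server as Host and toggles other players between Ready and Not Ready.
; Client update requests call a server send function, while a separate event has the lobby game mode update all player widgets.
; Incoming name and status lists go to player controller 0, which clears and rebuilds its lobby list.
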(event `BlueprintUpdateReadyStatus`
  (params (IsServer :type Boolean))
  (if IsServer
    (set `self.BlueprintPlayerReadyStatus` "Host")
    (elif (`KismetStringLibrary.EqualEqual_StrStr` (`self.BlueprintPlayerReadyStatus`) "Ready")
      (set `self.BlueprintPlayerReadyStatus` "Not Ready")
      (else
        (set `self.BlueprintPlayerReadyStatus` "Ready")))))

(event `Client_SendLobbyWidgetUpdateToServer`
  (`self.Server_SendLobbyWidgetUpdate`))

(event `Server_SendLobbyWidgetUpdate`
  (`/Game/Blueprints/Starmark_GameMode_Lobby_Blueprint.UpdatePlayerLobbyWidgets` (cast `/Game/Blueprints/Starmark_GameMode_Lobby_Blueprint` (`GameplayStatics.GetGameMode`) :!pure true)))

(event `Server_UpdatePlayerLobbyWidget`
  (params (PlayerNames :type "Array of String") (PlayerReadyStatuses :type "Array of String"))
  (bind _asplayer_controller_lobby_blueprint (cast `/Game/Blueprints/PlayerController_Lobby_Blueprint` (`GameplayStatics.GetPlayerController` 0))
    (:`then`
      (`PlayerController_Lobby.UpdatePlayersInLobby` _asplayer_controller_lobby_blueprint PlayerNames PlayerReadyStatuses true))
    (:`CastFailed`
      (`KismetSystemLibrary.PrintString` "Cast to PlayerController_Lobby Failed!" true true (struct :`R` 1.0 :`A` 1.0) 15.0))))

(fn `UserConstructionScript`)