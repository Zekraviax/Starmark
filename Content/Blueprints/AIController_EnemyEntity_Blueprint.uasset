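; AI controller for enemy entities that plays their move-and-attack turn in Starmark's tile-based combat.
; On possess it runs a behavior tree; step two paths to the target, trimming path points to the avatar's tile-move allowance.
; Tick uses a resettable DoOnce to trigger the range check when movement stops.
; That check picks a random attack, then launches it through the GameMode if path distance is in range, otherwise ends the turn.
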(event `self.ReceiveTick`
  (params (DeltaSeconds :type "Float (single-precision)"))
  (`/Engine/EditorBlueprintResources/StandardMacros.IsValid` (`self.SelfEntityReference`)
    (:`Is Valid`
      (if (<= (`KismetMathLibrary.VSize` (`self.GetVelocity` (`self.SelfEntityReference`))) 0.0)
        (`/Engine/EditorBlueprintResources/StandardMacros.DoOnce` true :!label _label
          (:`Completed`
            (`self.StepThree_CheckIfTargetIsInRange`)))
        (else
          (goto _label :!via `Reset`))))))

(event `self.ReceivePossess`
  (params (PossessedPawn :type "Pawn Object Reference"))
  (`self.RunBehaviorTree` "/Game/Blueprints/CharacterPathfindingAI/CharacterPathfindingAI_BehaviourTree.CharacterPathfindingAI_BehaviourTree")
  (`self.SetReplicateMovement` true))

(event `self.StepTwo_MoveToTarget`
  (bind _selfentityreference (`self.SelfEntityReference`))
  (bind _returnvalue (`self.K2_GetActorLocation` _selfentityreference))
  (`parent.StepTwo_MoveToTarget`)
  (bind _returnvalue_2 (`NavigationSystemV1.FindPathToLocationSynchronously` _returnvalue (`self.K2_GetActorLocation` (`self.CurrentTarget`)) self null))
  (bind _pathpoints (`NavigationPath.PathPoints` _returnvalue_2))
  (bind _returnvalue_3 (`KismetArrayLibrary.Array_Length` _pathpoints))
  (if (not (and (`NavigationPath.IsValid` _returnvalue_2) (> _returnvalue_3 0)))
    (`KismetSystemLibrary.PrintText` (`KismetTextLibrary.Conv_StringToText` (`NavigationPath.GetDebugString` _returnvalue_2)) true true (struct :`R` 1.0 :`A` 1.0) 15.0)
    (else
      (bind _returnvalue_4 (`KismetArrayLibrary.Array_LastIndex` _pathpoints))
      (bind _output (`|GetArrayItem` _pathpoints _returnvalue_4))
      (if (not (== _returnvalue _output :`ErrorTolerance` 0.1))
        (while (> _returnvalue_3 (`.CurrentTileMoves` (break `NetscapeExplorer_Struct` (`Character_Pathfinder.AvatarData` _selfentityreference))))
          (`KismetArrayLibrary.Array_Remove` _pathpoints _returnvalue_4))
        (`self.MoveToLocation` _output -1.0 false true false true null)))))

(event `StepThree_CheckIfTargetIsInRange_1`
  (bind ((`CurrentAttacks` _currentattacks) (`Attacks` _attacks)) (break `NetscapeExplorer_Struct` (`Character_Pathfinder.AvatarData` (`self.SelfEntityReference`))))
  (bind (_datatable _rowname) (break `DataTableRowHandle` (`|GetArrayItem` _attacks (`KismetMathLibrary.RandomIntegerInRange` 0 (`KismetArrayLibrary.Array_LastIndex` _attacks)))))
  (bind _returnvalue (`|GetDataTableRow` _datatable _rowname)
    (:`then`
      (bind _output_get (set `self.CurrentAttack` _returnvalue))
      (bind _returnvalue_2 (`NavigationSystemV1.FindPathToLocationSynchronously` (`self.K2_GetActorLocation` (`self.SelfEntityReference`)) (`self.K2_GetActorLocation` (`self.CurrentTarget`)) self null))
      (bind ((`Name` _name) (`BaseRange` _baserange)) (break `Avatar_AttackStruct` _output_get))
      (if (<= (/ (`KismetMathLibrary.FTrunc` (`NavigationPath.GetPathLength` _returnvalue_2)) 200) _baserange)
        (`Starmark_GameMode.Server_LaunchAttack` (cast `Starmark_GameMode` (`GameplayStatics.GetGameMode`) :!pure true) (`self.SelfEntityReference`) (`self.CurrentTarget`) _name)
        (else
          (`Starmark_GameState.AvatarEndTurn` (cast `Starmark_GameState` (`GameplayStatics.GetGameState`) :!pure true)))))))

(fn `UserConstructionScript`)