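; A player pawn, named as a flying pawn, that moves through a FloatingPawnMovement component.
; The MoveForward and MoveRight axis inputs add movement along the forward and right vectors of the control rotation, scaled by the axis value.
; Only the yaw of that rotation is used, so this input stays horizontal regardless of pitch.
; The graphs contain no look or vertical movement input, and the construction script is empty.
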(event `InputAxis|MoveForward`
  (params (AxisValue :type "Float (single-precision)"))
  (if (!= AxisValue 0.0)
    (`PawnMovementComponent.AddInputVector` (`self.FloatingPawnMovement`) (* (`KismetMathLibrary.GetForwardVector` (`KismetMathLibrary.MakeRotator` 0.0 0.0 (.yaw (`self.GetControlRotation`)))) AxisValue) false)))

(event `InputAxis|MoveRight`
  (params (AxisValue :type "Float (single-precision)"))
  (if (!= AxisValue 0.0)
    (`PawnMovementComponent.AddInputVector` (`self.FloatingPawnMovement`) (* (`KismetMathLibrary.GetRightVector` (`KismetMathLibrary.MakeRotator` 0.0 0.0 (.yaw (`self.GetControlRotation`)))) AxisValue) false)))

(fn `UserConstructionScript`)