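; Battle game mode Blueprint that handles multiplayer player login and session teardown.
; On login it expects one player in DevLevel maps and two otherwise, then passes the battle player controller to OnPlayerPostLogin.
; A custom event waits briefly, destroys the session, and on success calls EndOfSession on each stored player controller.
; HandleStartingNewPlayer only prints a debug message.
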(event `self.K2_PostLogin`
  (params (NewPlayer :type "PlayerController Object Reference"))
  ;[1 1 1] Mtultiplayer Functions
  (bind _returnvalue (`GameplayStatics.GetCurrentLevelName` true))
  (if (`KismetStringLibrary.Contains` _returnvalue "DevLevel")
    (set `self.ExpectedPlayers` 1)
    (else
      (set `self.ExpectedPlayers` 2)))
  (bind _asplayer_controller_battle_blueprint (cast `/Game/Blueprints/PlayerController_Battle_Blueprint` NewPlayer))
  (`self.OnPlayerPostLogin` _asplayer_controller_battle_blueprint))

(event `CustomEvent`
  ;[1 1 1] Mtultiplayer Functions
  (`KismetSystemLibrary.Delay` 3.0)
  (`DestroySessionCallbackProxy.DestroySession` (`GameplayStatics.GetPlayerController` 0)
    (:`OnSuccess`
      (for _array_element (`self.PlayerControllerReferences`)
        (bind _asplayer_controller_battle_blueprint (cast `/Game/Blueprints/PlayerController_Battle_Blueprint` _array_element))
        (`/Game/Blueprints/PlayerController_Battle_Blueprint.EndOfSession` _asplayer_controller_battle_blueprint)))))

(event `self.HandleStartingNewPlayer`
  (params (NewPlayer :type "PlayerController Object Reference"))
  ;[1 1 1] Mtultiplayer Functions
  (`KismetSystemLibrary.PrintString` "Starmark_GameMode_Battle_Blueprint / EventHandleStartingNewPlayer / A new player is ready to be handled" true true (struct :`G` 0.66 :`B` 1.0 :`A` 1.0) 5.0))

(fn `UserConstructionScript`)