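; World grid actor meant to spawn a field of Actor_GridTile_Blueprint tiles, though that logic is currently disconnected and BeginPlay does nothing.
; The unused nested loops span GridX and GridY around the world origin, placing tiles at fixed spacing at the actor's height.
; Each spawned tile would be stored in GridTilesArray.
; The construction script is empty.
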(event `self.ReceiveBeginPlay`)

(fn `UserConstructionScript`)